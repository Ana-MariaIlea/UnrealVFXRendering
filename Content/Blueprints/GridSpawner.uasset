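; GridSpawner is a framerate benchmark actor that spawns a square grid of galaxy systems in either a once or infinite variant.
; BeginPlay adds the HUD, shows the cursor and binds to BP_FramerateTrackerActor to collect samples.
; SpawnGalaxies configures and starts the tracker, then fills the grid on the XZ plane.
; After a fixed delay, it saves the samples to a FramerateSaveGame slot and quits the game.
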(event Custom|SpawnGalaxies
  (params (IndexNumber :type Integer) (IsOnceSystem :type Boolean))
  (Variables|Default|SetIs%20Once%20System IsOnceSystem)
  (if (Variables|Default|GetIs%20Once%20System)
    (Variables|Default|SetGalaxiClass "/Game/Blueprints/GalaxyBlueprintOnce.GalaxyBlueprintOnce_C")
    (else
      (Variables|Default|SetGalaxiClass "/Game/Blueprints/GalaxyBlueprintInfinite.GalaxyBlueprintInfinite_C")))
  (Default|SetTestVariables (Variables|Default|GetFramerateTrackerActor) (* IndexNumber IndexNumber) (Variables|Default|GetIs%20Once%20System))
  (Variables|Default|SetLastIndex IndexNumber)
  (Default|StartTrackingFramete (Variables|Default|GetFramerateTrackerActor))
  (for _index (range 0 (Variables|Default|GetLastIndex))
    (for _index_2 (range 0 (Variables|Default|GetLastIndex))
      (bind _returnvalue (Game|SpawnActorfromClass (Variables|Default|GetGalaxiClass) (Math|Transform|MakeTransform (Math|Vector|MakeVector (Math|Conversions|ToFloat(Integer) (* _index 6000)) 0.0 (Math|Conversions|ToFloat(Integer) (* _index_2 4000))) "0, 0, 0" "1.000000,1.000000,1.000000") "Undefined" 0 0))
      (if (Variables|Default|GetIs%20Once%20System)
        (bind _asgalaxy_blueprint_once (Utilities|Casting|CastToGalaxyBlueprintOnce _returnvalue))
        (Utilities|Array|Add (Variables|Default|GetGalaxySystemsOnce) _asgalaxy_blueprint_once)
        (else
          (bind _asgalaxy_blueprint_infinite (Utilities|Casting|CastToGalaxyBlueprintInfinite _returnvalue))
          (Utilities|Array|Add (Variables|Default|GetGalaxySystesInfinite) _asgalaxy_blueprint_infinite)))))
  (Utilities|FlowControl|Delay 2e+01)
  (bind _returnvalue_2 (SaveGame|CreateSaveGameObject "/Game/Blueprints/FramerateSaveGame.FramerateSaveGame_C"))
  (Variables|/Game/Blueprints/FramerateSaveGame.FramerateSaveGame_C|SetFramerateStructure _returnvalue_2 (Variables|Default|GetFramerateStructure))
  (SaveGame|SaveGametoSlot _returnvalue_2 "FrameRateSaveGame")
  (Game|QuitGame 0 "Quit" false))

(event Custom|FramerateIncrease
  (params (NewStructureelement :type Framerate%20Structure%20Structure))
  (Utilities|Array|Add (Variables|Default|GetFramerateStructure) NewStructureelement))

(event EventBeginPlay
  (bind _returnvalue (UserInterface|CreateWidget "/Game/Blueprints/HUD.HUD_C"))
  (UserInterface|Viewport|AddtoViewport _returnvalue 0)
  (bind _returnvalue_2 (Actor|GetActorOfClass "/Game/Blueprints/BP_FramerateTrackerActor.BP_FramerateTrackerActor_C"))
  (bind _output_get (Variables|Default|SetFramerateTrackerActor _returnvalue_2))
  (EventDispatchers|BindEventtoFramerateTracker _output_get (delegate Custom|FramerateIncrease))
  (Variables|/Script/Engine.PlayerController|SetbShowMouseCursor (Game|GetPlayerController (Variables|/Script/Engine.Pawn|GetPlayerState (Game|Player|GetPlayerPawn 0))) true))

(fn ConstructionScript)