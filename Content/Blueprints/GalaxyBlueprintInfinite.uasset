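; Galaxy actor that plays a collision between two particle-system galaxies on BeginPlay.
; Latent MoveComponentTo calls bring both to the relative origin over Time, then out to opposite offsets, using Galaxy1's rotation for both.
; Curl-noise parameters spike half a second before they meet and reset after Galaxy2's second move.
; Despite the "Infinite" name, the sequence runs once: the delayed re-entries into the outward moves are unconnected.
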(event EventBeginPlay
  (bind _galaxy1 (Variables|Default|GetGalaxy1))
  (bind _galaxy1_2 (Variables|Default|GetGalaxy1))
  (bind _galaxy1_3 (Variables|Default|GetGalaxy1))
  (bind _galaxy1_4 (Variables|Default|GetGalaxy1))
  (bind _relativerotation (Variables|/Script/Engine.SceneComponent|GetRelativeRotation _galaxy1_4))
  (bind _relativerotation_2 (Variables|/Script/Engine.SceneComponent|GetRelativeRotation _galaxy1_2))
  (bind _relativerotation_3 (Variables|/Script/Engine.SceneComponent|GetRelativeRotation _galaxy1))
  (bind _relativerotation_4 (Variables|/Script/Engine.SceneComponent|GetRelativeRotation _galaxy1_3))
  (bind (_roll _pitch _yaw) (Math|Rotator|BreakRotator _relativerotation))
  (bind (_roll_2 _pitch_2 _yaw_2) (Math|Rotator|BreakRotator _relativerotation_2))
  (bind (_roll_3 _pitch_3 _yaw_3) (Math|Rotator|BreakRotator _relativerotation_3))
  (bind (_roll_4 _pitch_4 _yaw_4) (Math|Rotator|BreakRotator _relativerotation_4))
  (Utilities|FlowControl|DelayUntilNextTick)
  (Utilities|FlowControl|Sequence
    (:then_0
      (Components|MoveComponentTo (Variables|Default|GetGalaxy1) "0, 0, 0" (Math|Rotator|MakeRotator _roll _pitch _yaw) false false (Variables|Default|GetTime) false)
      (Components|MoveComponentTo (Variables|Default|GetGalaxy1) "1500.000000, 0,1000.000000" (Math|Rotator|MakeRotator _roll_4 _pitch_4 _yaw_4) false false (Variables|Default|GetTime) false))
    (:then_1
      (Components|MoveComponentTo (Variables|Default|GetGalaxy2) "0, 0, 0" (Math|Rotator|MakeRotator _roll_2 _pitch_2 _yaw_2) false false (Variables|Default|GetTime) false)
      (Components|MoveComponentTo (Variables|Default|GetGalaxy2) "-1500.000000, 0,-1000.000000" (Math|Rotator|MakeRotator _roll_3 _pitch_3 _yaw_3) false false (Variables|Default|GetTime) false)
      (CallFunction|ChangeVFXParameterstoNormal (Variables|Default|GetGalaxy1))
      (CallFunction|ChangeVFXParameterstoNormal (Variables|Default|GetGalaxy2)))
    (:then_2
      (Utilities|FlowControl|Delay (+ (Variables|Default|GetTime) -0.5))
      (CallFunction|ChangeVFXParameters (Variables|Default|GetGalaxy1))
      (CallFunction|ChangeVFXParameters (Variables|Default|GetGalaxy2)))))

(fn ConstructionScript)

(fn ChangeVFXParameters
  (params (ParticleSystem :type Niagara%20Component%20Object%20Reference))
  (Effects|Components|ParticleSystem|SetFloatParameter ParticleSystem "SmallPariclesCurlNoiseStength" 2e+04)
  (Effects|Components|ParticleSystem|SetFloatParameter ParticleSystem "SmallPariclesCurlNoiseFrequency" 1e+02)
  (Effects|Components|ParticleSystem|SetFloatParameter ParticleSystem "BigPariclesCurlNoiseStength" 2e+04)
  (Effects|Components|ParticleSystem|SetFloatParameter ParticleSystem "BigPariclesCurlNoiseFrequency" 5e+01)
  (Effects|Components|ParticleSystem|SetFloatParameter ParticleSystem "CloudCurlNoiseStength" 5e+03)
  (Effects|Components|ParticleSystem|SetFloatParameter ParticleSystem "CloudCurlNoiseFrequency" 1e+01))

(fn ChangeVFXParameterstoNormal
  (params (ParticleSystem :type Niagara%20Component%20Object%20Reference))
  (Effects|Components|ParticleSystem|SetFloatParameter ParticleSystem "SmallPariclesCurlNoiseStength" 1e+02)
  (Effects|Components|ParticleSystem|SetFloatParameter ParticleSystem "SmallPariclesCurlNoiseFrequency" 5e+01)
  (Effects|Components|ParticleSystem|SetFloatParameter ParticleSystem "BigPariclesCurlNoiseStength" 2e+02)
  (Effects|Components|ParticleSystem|SetFloatParameter ParticleSystem "BigPariclesCurlNoiseFrequency" 1e+02)
  (Effects|Components|ParticleSystem|SetFloatParameter ParticleSystem "CloudCurlNoiseStength" 1e+02)
  (Effects|Components|ParticleSystem|SetFloatParameter ParticleSystem "CloudCurlNoiseFrequency" 0.001))