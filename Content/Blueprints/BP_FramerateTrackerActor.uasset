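; Actor for framerate benchmarking of particle systems, recording FPS against system count and loop type (Once or Infinite).
; On BeginPlay it loads the FrameRateSaveGame slot and replays each saved entry through TrackFramerate.
; Tick derives FPS from delta time, and FramerateTracking packages it with the test settings and elapsed seconds for CallFramerateTracker.
; The half-second sampling timer is disconnected and StartTrackingFramete is empty, so nothing here triggers sampling.
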(event Custom|FramerateTracking
  (Default|CallFramerateTracker (Utilities|Struct|MakeFramerateStructure (Variables|Default|GetSystemType) (Variables|Default|GetNumberOfSystems) (Variables|Default|GetSeconds) (Variables|Default|GetFramerateVariable)))
  (Variables|Default|SetSeconds (+ (Variables|Default|GetSeconds) 0.5)))

(event Custom|SetTestVariables
  (params (NumberOfSystems :type Integer) (IsSystemOnce :type Boolean))
  (if (== NumberOfSystems 0)
    (Variables|Default|SetNumberOfSystems 1)
    (else
      (Variables|Default|SetNumberOfSystems NumberOfSystems)))
  (if IsSystemOnce
    (Variables|Default|SetSystemType "Once")
    (else
      (Variables|Default|SetSystemType "Infinite"))))

(event Custom|SetNumberOfParticles
  (params (ParticlesNumber :type Integer))
  (Variables|Default|SetNumberOfParticles ParticlesNumber))

(event Custom|StartTrackingFramete)

(event EventBeginPlay
  (bind _returnvalue (SaveGame|LoadGamefromSlot "FrameRateSaveGame"))
  (bind _asframerate_save_game (Utilities|Casting|CastToFramerateSaveGame _returnvalue))
  (Development|PrintString "Hello")
  (for _array_element (Variables|/Game/Blueprints/FramerateSaveGame.FramerateSaveGame_C|GetFramerateStructure _asframerate_save_game)
    (Class|FramerateTrackerActor|TrackFramerate (.LoopBehavior (Utilities|Struct|BreakFramerateStructure _array_element)) (.NumberOfSystems (Utilities|Struct|BreakFramerateStructure _array_element)) (.Seconds (Utilities|Struct|BreakFramerateStructure _array_element)) (.Framerate (Utilities|Struct|BreakFramerateStructure _array_element)))))

(event EventTick
  (params (DeltaSeconds :type Float%20%28single-precision%29))
  (Variables|Default|SetFramerateVariable (/ 1.0 DeltaSeconds)))

(fn ConstructionScript)